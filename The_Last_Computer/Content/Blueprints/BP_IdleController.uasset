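; Player controller for an isometric camera that shows the cursor, enables click events and drives the BP_IsoCam pawn.
; Keyboard axes move the pawn along its local axes, at a clamped speed that scales with spring arm length.
; A screen-edge macro turns cursor position near viewport borders into local pawn offsets.
; The mouse wheel steps a clamped zoom multiplier, and Tick smoothly interpolates the arm length toward it.
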(event `self.ReceiveTick`
  (params (DeltaSeconds :type "Float (single-precision)"))
  ;[0.2775 1 0.2124] Tick Events
  (`self.UpdateCameraZoom`))

(event `self.ReceiveBeginPlay`
  (`self.CastReferences`
    (:`ReturnNode`
      (set `self.bShowMouseCursor` true)
      (set `SpringArmComponent.TargetArmLength` (* (`self.ZoomStep`) (`self.ZoomMultiplier`)) (`/Game/Blueprints/BP_IsoCam.SpringArm` (`self.CameraPawnReference`)))
      (set `self.bEnableClickEvents` true))))

(event `InputAxisKey|MouseX`
  (params (AxisValue :type "Float (single-precision)"))
  ;[1 1 1] Mouse Edge Screen Movement
  (bind (_deltaxspeed _deltayspeed) (`self.ScreenEdgeMovement` :!label _label)
    (:`ReturnNode`
      (`self.K2_AddActorLocalOffset` (`self.CameraPawnReference`) (`KismetMathLibrary.MakeVector` _deltaxspeed _deltayspeed) false false))))

(event `InputAxisKey|MouseY`
  (params (AxisValue :type "Float (single-precision)"))
  ;[1 1 1] Mouse Edge Screen Movement
  (goto _label :!via `MouseY`))

(event `InputAxis|MoveForward`
  (params (AxisValue :type "Float (single-precision)"))
  (bind _camerapawnreference (`self.CameraPawnReference`))
  ;[1 1 1] Vertical Camera Movement Keyboard
  (`self.K2_SetActorTransform` _camerapawnreference (`self.MovementX` AxisValue (`self.MovementSpeedCalculation`) (`self.MoveSensitivity`) _camerapawnreference) false false))

(event `InputAxis|MoveRight`
  (params (AxisValue :type "Float (single-precision)"))
  (bind _camerapawnreference (`self.CameraPawnReference`))
  ;[1 1 1] Horizontal Camera Movement Keyboard
  (`self.K2_SetActorTransform` _camerapawnreference (`self.MovementY` AxisValue (`self.MovementSpeedCalculation`) (`self.MoveSensitivity`) _camerapawnreference) false false))

(event `Key|MouseScrollUp`
  (params (Key :type "Key Structure"))
  (bind (_zoombounds_x _zoombounds_y) (`KismetMathLibrary.BreakVector2D` (`self.ZoomBounds`)))
  (:`Pressed`
    (`/Engine/EditorBlueprintResources/StandardMacros.IncrementFloat` (`self.ZoomMultiplier`)
      (:`  `
        (set `self.ZoomMultiplier` (`KismetMathLibrary.FClamp` (`self.ZoomMultiplier`) _zoombounds_x _zoombounds_y))))))

(event `Key|MouseScrollDown`
  (params (Key :type "Key Structure"))
  (bind (_zoombounds_x _zoombounds_y) (`KismetMathLibrary.BreakVector2D` (`self.ZoomBounds`)))
  (:`Pressed`
    (`/Engine/EditorBlueprintResources/StandardMacros.DecrementFloat` (`self.ZoomMultiplier`)
      (:`  `
        (set `self.ZoomMultiplier` (`KismetMathLibrary.FClamp` (`self.ZoomMultiplier`) _zoombounds_x _zoombounds_y))))))

(fn `MovementSpeedCalculation`
  (returns (MoveSensitivity :type "Float (double-precision)"))
  (return (`KismetMathLibrary.FClamp` (/ (`SpringArmComponent.TargetArmLength` (`/Game/Blueprints/BP_IsoCam.SpringArm` (`self.CameraPawnReference`))) 100.0) 5.0 20.0)))

(fn `UpdateCameraZoom`
  (locals (TempCurrentZoom :type "Float (double-precision)"))
  (set `local.TempCurrentZoom` (`SpringArmComponent.TargetArmLength` (`/Game/Blueprints/BP_IsoCam.SpringArm` (`self.CameraPawnReference`))))
  (set `SpringArmComponent.TargetArmLength` (`KismetMathLibrary.FInterpTo` (`local.TempCurrentZoom`) (* (`self.ZoomStep`) (`self.ZoomMultiplier`)) (`GameplayStatics.GetWorldDeltaSeconds`) 3.0) (`/Game/Blueprints/BP_IsoCam.SpringArm` (`self.CameraPawnReference`))))

(fn `UserConstructionScript`)