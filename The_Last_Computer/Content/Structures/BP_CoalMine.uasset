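; Clickable coal mine structure that starts coal gathering on the player stats object, cast from the game instance.
; Clicking the cube sets the gathering flag, starts a retriggerable delay and arms a timer, both using the coal gather delay.
; The timer re-arms itself, and UpdateTimer copies its elapsed time into the stats, or zero when not gathering.
; No coal is awarded here, and nothing follows either delay.
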(event `self.ReceiveBeginPlay`
  (bind _asbp_player_stats (cast `/Game/Blueprints/BP_PlayerStats` (`GameplayStatics.GetGameInstance`)))
  (set `self.PlayerRef` _asbp_player_stats))

(event `self.ReceiveTick`
  (params (DeltaSeconds :type "Float (single-precision)")))

(event `self.Cube.OnClicked`
  (params (TouchedComponent :type "PrimitiveComponent Object Reference") (ButtonPressed :type "Key Structure"))
  (set `/Game/Blueprints/BP_PlayerStats.IsGatheringCoal?` true (`self.PlayerRef`))
  (`|ExecutionSequence`
    (:`then_0`
      (`KismetSystemLibrary.RetriggerableDelay` (`/Game/Blueprints/BP_PlayerStats.CoalGatherDelay` (`self.PlayerRef`))))
    (:`then_1`
      (`self.Timer`)
      (`self.Update Timer`)
      (`KismetSystemLibrary.PrintString` (`KismetStringLibrary.Conv_DoubleToString` (`/Game/Blueprints/BP_PlayerStats.CoalDelaySeconds` (`self.PlayerRef`)))))))

(event `Timer`
  (bind _returnvalue (`KismetSystemLibrary.K2_SetTimerDelegate` (delegate `Timer`) (`/Game/Blueprints/BP_PlayerStats.CoalGatherDelay` (`self.PlayerRef`)))))

(event `Update Timer`
  (bind _playerref (`self.PlayerRef`))
  (if (`/Game/Blueprints/BP_PlayerStats.IsGatheringCoal?` _playerref)
    (set `/Game/Blueprints/BP_PlayerStats.CoalDelaySeconds` (`KismetSystemLibrary.K2_GetTimerElapsedTimeHandle` (stale `Timer` _returnvalue)) (`self.PlayerRef`))
    (`KismetSystemLibrary.Delay` 0.1)
    (else
      (set `/Game/Blueprints/BP_PlayerStats.CoalDelaySeconds` 0.0 _playerref))))

(fn `UserConstructionScript`)