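; BP_Computer is a computer structure that reveals its Cone component once the player has at least ten coal.
; On BeginPlay it casts the Game Instance to BP_PlayerStats and caches it as PlayerRef.
; Tick polls CoalAmount and sets the cone visible at that threshold, with no logic to hide it again.
; The construction script and StatsRef function are empty.
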(event `self.ReceiveBeginPlay`
  (bind _asbp_player_stats (cast `/Game/Blueprints/BP_PlayerStats` (`GameplayStatics.GetGameInstance`)))
  (set `self.PlayerRef` _asbp_player_stats))

(event `self.ReceiveTick`
  (params (DeltaSeconds :type "Float (single-precision)"))
  (if (>= (`/Game/Blueprints/BP_PlayerStats.CoalAmount` (`self.PlayerRef`)) 10.0)
    (`SceneComponent.SetVisibility` (`self.Cone`) true false)))

(fn `StatsRef`
  (returns (PlayerStats :type "/Game/Blueprints/BP_PlayerStats Object Reference"))
  (return null))

(fn `UserConstructionScript`)