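; BP_IdleController is a controller that shows the mouse cursor and pans the BP_IsoCam camera pawn.
; MoveForward and MoveRight inputs move the pawn along its local axes, with speed scaled by clamped spring arm length and MoveSensitivity.
; Mouse movement feeds ScreenEdgeMovement, which turns a cursor near the viewport border into a local offset scaled only by MoveSensitivity.
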(event `self.ReceiveBeginPlay`
  (`self.CastReferences`
    (:`ReturnNode`
      (set `self.bShowMouseCursor` true))))

(event `InputAxisKey|MouseX`
  (params (AxisValue :type "Float (single-precision)"))
  ;[1 1 1] Mouse Edge Screen Movement
  (bind (_deltaxspeed _deltayspeed) (`self.ScreenEdgeMovement` :!label _label)
    (:`ReturnNode`
      (`self.K2_AddActorLocalOffset` (`self.CameraPawnReference`) (`KismetMathLibrary.MakeVector` _deltaxspeed _deltayspeed) false false))))

(event `InputAxisKey|MouseY`
  (params (AxisValue :type "Float (single-precision)"))
  ;[1 1 1] Mouse Edge Screen Movement
  (goto _label :!via `MouseY`))

(event `InputAxis|MoveForward`
  (params (AxisValue :type "Float (single-precision)"))
  (bind _camerapawnreference (`self.CameraPawnReference`))
  (`self.K2_SetActorTransform` _camerapawnreference (`self.MovementX` AxisValue (`self.MovementSpeedCalculation`) (`self.MoveSensitivity`) _camerapawnreference) false false))

(event `InputAxis|MoveRight`
  (params (AxisValue :type "Float (single-precision)"))
  (bind _camerapawnreference (`self.CameraPawnReference`))
  (`self.K2_SetActorTransform` _camerapawnreference (`self.MovementY` AxisValue (`self.MovementSpeedCalculation`) (`self.MoveSensitivity`) _camerapawnreference) false false))

(fn `MovementSpeedCalculation`
  (returns (MoveSensitivity :type "Float (double-precision)"))
  (return (`KismetMathLibrary.FClamp` (/ (`SpringArmComponent.TargetArmLength` (`/Game/BP_IsoCam.SpringArm` (`self.CameraPawnReference`))) 100.0) 5.0 20.0)))

(fn `UserConstructionScript`)